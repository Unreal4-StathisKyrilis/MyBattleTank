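; Main menu HUD Blueprint that creates the main menu widget when play begins.
; BeginPlay passes the new widget to a Game and UI input mode for player 0 as the focus target, keeping the cursor visible during capture.
; The AddToViewport call is disconnected, so this graph never displays the widget itself.
; Options menu creation, alternative input modes and "Settings" save-game loading are also unwired leftovers.
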(event `self.ReceiveBeginPlay`
  (bind _returnvalue (`|CreateWidget` "/Game/mainMenu/_BluePrints/MainMenu_Widget.MainMenu_Widget_C"))
  (`WidgetBlueprintLibrary.SetInputMode_GameAndUIEx` (`GameplayStatics.GetPlayerController` 0) _returnvalue "DoNotLock" false))

(event `self.ReceiveDrawHUD`
  (params (SizeX :type Integer) (SizeY :type Integer)))

(fn `UserConstructionScript`)