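; Player-controllable tank Blueprint that drives, aims with a gimbal camera rig and fires.
; On BeginPlay it hands barrel and turret to TankAiming and both tracks, with left and right swapped, to TankMovement.
; Input axes rotate the azimuth gimbal and spring arm or send movement intents, while Fire calls TankAiming and plays an explosion sound.
; The construction script assigns meshes and configures track physical material and hit notifications.
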(event `self.ReceiveBeginPlay`
  (`TankAimingComponent.Initialise` (`self.TankAiming`) (`self.Barrel`) (`self.Turret`))
  (`TankMovementComponent.Initialise` (`self.TankMovement`) (`self.RightTrack`) (`self.LeftTrack`))
  (`TankMovementComponent.Initialise` (`self.TankMovement`) (`self.RightTrack`) (`self.LeftTrack`)))

(event `InputAxis|AimAzimuth`
  (params (AxisValue :type "Float (single-precision)"))
  ;[1 1 1] Ballistics Input Binding
  (`SceneComponent.K2_AddLocalRotation` (`self.Azimuth Gimbal`) (`KismetMathLibrary.MakeRotator` 0.0 0.0 AxisValue) false false))

(event `InputAxis|MoveFowrard`
  (params (AxisValue :type "Float (single-precision)"))
  ;[1 1 1] Movement Input Binding
  (`TankMovementComponent.IntendMoveForward` (`self.TankMovement`) AxisValue))

(event `InputAxis|AimElevation`
  (params (AxisValue :type "Float (single-precision)"))
  ;[1 1 1] Ballistics Input Binding
  (`SceneComponent.K2_AddLocalRotation` (`self.SpringArm`) (`KismetMathLibrary.MakeRotator` 0.0 AxisValue) false false))

(event `InputAxis|TurnRight`
  (params (AxisValue :type "Float (single-precision)"))
  ;[1 1 1] Movement Input Binding
  (`TankMovementComponent.IntendTurnRight` (`self.TankMovement`) AxisValue))

(event `InputAction|Fire`
  (params (Key :type "Key Structure"))
  ;[1 1 1] Ballistics Input Binding
  (:`Pressed`
    (`TankAimingComponent.Fire` (`self.TankAiming`))
    (`GameplayStatics.PlaySoundAtLocation` "/Game/StarterContent/Audio/Explosion01.Explosion01" (`SceneComponent.GetSocketLocation` (`self.Tank`) "Turret") (struct) 1.0 1.0 0.0 null null null)))

(fn `UserConstructionScript`
  (bind _lefttrack (`self.LeftTrack`))
  (bind _righttrack (`self.RightTrack`))
  (`StaticMeshComponent.SetStaticMesh` (`self.Turret`) "/Game/3D/Tank/tank_fbx_Turret.tank_fbx_Turret")
  (`StaticMeshComponent.SetStaticMesh` (`self.Barrel`) "/Game/3D/Tank/tank_fbx_Barrel.tank_fbx_Barrel")
  (`StaticMeshComponent.SetStaticMesh` _lefttrack "/Game/3D/Tank/tank_fbx_Track.tank_fbx_Track")
  (`StaticMeshComponent.SetStaticMesh` _righttrack "/Game/3D/Tank/tank_fbx_Track.tank_fbx_Track")
  (`PrimitiveComponent.SetPhysMaterialOverride` _lefttrack "/Game/3D/Tank/Track.Track")
  (`PrimitiveComponent.SetPhysMaterialOverride` _righttrack "/Game/3D/Tank/Track.Track")
  (`PrimitiveComponent.SetNotifyRigidBodyCollision` (`self.LeftTrack`) true)
  (`PrimitiveComponent.SetNotifyRigidBodyCollision` (`self.RightTrack`) true))